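; An interactable stand actor that lets the player toggle an on-screen image widget with E while overlapping it.
; Overlap begin enables input and copies the stand's Image value into the FirstPersonCharacter's ImageIndex, presumably for the widget to read.
; A FlipFlop on E alternately creates and removes the widget.
; Overlap end disables input and removes the widget without resetting the FlipFlop.
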(event `Key|E`
  (params (Key :type "Key Structure"))
  ;[1 1 1] interaction
  (:`Pressed`
    (`/Engine/EditorBlueprintResources/StandardMacros.FlipFlop`
      (:`A`
        (bind _returnvalue (`|CreateWidget` "/Game/WBP/WBP_img.WBP_img_C"))
        (`UserWidget.AddToViewport` _returnvalue 0))
      (:`B`
        (`Widget.RemoveFromParent` _returnvalue :!label _label)))))

(event `self.ReceiveActorBeginOverlap`
  (params (OtherActor :type "Actor Object Reference"))
  ;[1 1 1] interaction
  (`self.EnableInput` (`GameplayStatics.GetPlayerController` 0))
  (bind _asfirst_person_character (cast `/Game/FirstPersonBP/Blueprints/FirstPersonCharacter` (`GameplayStatics.GetPlayerCharacter` 0)))
  (set `/Game/FirstPersonBP/Blueprints/FirstPersonCharacter.image_index` (`self.image`) _asfirst_person_character))

(event `self.ReceiveActorEndOverlap`
  (params (OtherActor :type "Actor Object Reference"))
  ;[1 1 1] interaction
  (`self.DisableInput` null)
  (goto _label))

(fn `UserConstructionScript`)